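; Paper2D skeleton enemy that walks forward, turns around when its attack box meets anything other than the player, and attacks BP_MainCharacter.
; Tick triggers attacks while the player is in range and applies damage once per swing at flipbook frame 20.
; Incoming damage interrupts attacks with a hit flipbook; at zero health it disables capsule collision, plays death and destroys itself.
; MoveProcess drives walk and idle flipbooks but has no caller here.
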(event OnComponentBeginOverlap(AttackBox)
  (params (OverlappedComponent :type Primitive%20Component%20Object%20Reference) (OtherActor :type Actor%20Object%20Reference) (OtherComp :type Primitive%20Component%20Object%20Reference) (OtherBodyIndex :type Integer) (bFromSweep :type Boolean) (SweepResult :type Hit%20Result%20Structure%20%28by%20ref%29))
  (if (== (Utilities|GetClass OtherActor) "/Game/Blueprints/BP_MainCharacter.BP_MainCharacter_C")
    (bind _asbp_main_character (Utilities|Casting|CastToBP_MainCharacter OtherActor))
    (for _array_element (Class|PrimitiveComponent|GetOverlappingComponents (Variables|/Game/Blueprints/BP_MainCharacter.BP_MainCharacter_C|GetHitBox _asbp_main_character))
      (if (== _array_element OverlappedComponent)
        (Variables|Default|SetInAttackZone true)))
    (else
      (Transformation|SetActorRotation (Math|Rotator|CombineRotators (Transformation|GetActorRotation) "0.000000,180.000000,0.000000")))))

(event OnComponentEndOverlap(AttackBox)
  (params (OverlappedComponent :type Primitive%20Component%20Object%20Reference) (OtherActor :type Actor%20Object%20Reference) (OtherComp :type Primitive%20Component%20Object%20Reference) (OtherBodyIndex :type Integer))
  (if (== (Utilities|GetClass OtherActor) "/Game/Blueprints/BP_MainCharacter.BP_MainCharacter_C")
    (Variables|Default|SetInAttackZone false)))

(event Custom|MoveProcess
  (if (not (Variables|Default|GetTaking%20Damage))
    (if (not (Variables|Default|GetIsAttacking))
      (Class|PawnMovementComponent|AddInputVector (Variables|Character|GetCharacterMovement) (Transformation|GetActorForwardVector) false)
      (Math|Float|CompareFloat (Math|Vector|VectorLength (Variables|/Script/Engine.MovementComponent|GetVelocity (Variables|Character|GetCharacterMovement))) 0.0
        (:>
          (Sprite|SetFlipbook (Variables|Default|GetSprite) "/Game/Assets/Skeleton/Walk/FB_Skeleton_Walk.FB_Skeleton_Walk"))
        (:==
          (Sprite|SetFlipbook (Variables|Default|GetSprite) "/Game/Assets/Skeleton/Idle/FB_Skeleton_Idle.FB_Skeleton_Idle"))))))

(event Custom|Attack
  (if (not (Variables|Default|GetTaking%20Damage))
    (Variables|Default|SetIsAttacking true)
    (Sprite|SetFlipbook (Variables|Default|GetSprite) "/Game/Assets/Skeleton/Attack/FB_Skeleton_Attack.FB_Skeleton_Attack")
    (Utilities|FlowControl|Delay (Class|PaperFlipbookComponent|GetFlipbookLength (Variables|Default|GetSprite)))
    (Variables|Default|SetIsAttacking false)
    (CallFunction|ResetHit)))

(event Custom|ResetHit
  (Utilities|FlowControl|DoOnce false) ; enters at Reset
)

(event EventBeginPlay
  (Variables|/Script/Engine.PrimitiveComponent|SetCanCharacterStepUpOn (Variables|Collision|GetCapsuleComponent) "ECB_Yes")
  (Development|SetHiddeninGame (Variables|Default|GetAttackBox) false false))

(event Game|Damage|EventAnyDamage
  (params (Damage :type Float%20%28single-precision%29) (DamageType :type Damage%20Type%20Object%20Reference) (InstigatedBy :type Controller%20Object%20Reference) (DamageCauser :type Actor%20Object%20Reference))
  (Components|Timeline|SetNewTime (Variables|Default|GetSprite) 0.0)
  (Variables|Default|SetIsAttacking false)
  (Variables|Default|SetTaking%20Damage true)
  (if (not (Variables|Default|GetisDying))
    (Variables|Default|SetHealth (- (Variables|Default|GetHealth) Damage))
    (Sprite|SetFlipbook (Variables|Default|GetSprite) "/Game/Assets/Skeleton/Hit/FB_Skeleton_Hit.FB_Skeleton_Hit")
    (Utilities|FlowControl|Delay (Class|PaperFlipbookComponent|GetFlipbookLength (Variables|Default|GetSprite)))
    (if (<= (Variables|Default|GetHealth) 0.0)
      (Variables|Default|SetisDying true)
      (Sprite|SetFlipbook (Variables|Default|GetSprite) "/Game/Assets/Skeleton/Death/FB_Skeleton_Death.FB_Skeleton_Death")
      (Collision|SetCollisionEnabled (Variables|Collision|GetCapsuleComponent) "NoCollision")
      (Utilities|FlowControl|Delay (Class|PaperFlipbookComponent|GetFlipbookLength (Variables|Default|GetSprite)))
      (Actor|DestroyActor)
      (else
        (Variables|Default|SetTaking%20Damage false)
        (Sprite|SetFlipbook (Variables|Default|GetSprite) "/Game/Assets/Skeleton/Idle/FB_Skeleton_Idle.FB_Skeleton_Idle")))))

(event EventTick
  (params (DeltaSeconds :type Float%20%28single-precision%29))
  (if (Variables|Default|GetInAttackZone)
    (CallFunction|Attack)
    (if (== (Class|PaperFlipbookComponent|GetPlaybackPositioninFrames (Variables|Default|GetSprite)) 20) :!label _label
      (if (not (Variables|Default|GetTaking%20Damage))
        (Utilities|FlowControl|DoOnce false
          (:Completed
            (CallFunction|HitCheck)))))
    (elif (Variables|Default|GetIsAttacking)
      (goto _label))))

(fn ConstructionScript)

(fn HitCheck
  (for _array_element (Collision|GetOverlappingActors (Variables|Default|GetAttackBox) "/Game/Blueprints/BP_MainCharacter.BP_MainCharacter_C" :!class /Script/Engine.PrimitiveComponent)
    (if (!= _array_element self)
      (bind _returnvalue (Game|Damage|ApplyDamage _array_element (Variables|Default|GetDamage) 0 self))
      (Development|PrintText (Utilities|Text|ToText(Float) _returnvalue "HalfToEven")))))