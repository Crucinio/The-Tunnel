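; Player character for a 2D flipbook side-scroller that runs, jumps, slides and fights BP_Skeleton enemies.
; Jumping uses input buffering and ledge grace time, while charge-limited slides shrink the capsule and knock skeletons upward.
; Attacks form a two-hit combo with frame-timed overlap damage, or a height-checked falling slam that spawns a shockwave on landing.
; Tick drives animation, slide and hit checks; damage triggers hit or death flipbooks, and destruction requests respawn from MainGameMode.
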(event Custom|ResetHit%201
  (Utilities|FlowControl|DoOnce false) ; enters at Reset
)

(event Custom|ResetHit%202
  (Utilities|FlowControl|DoOnce false) ; enters at Reset
)

(event EventBeginPlay
  (Development|SetHiddeninGame (Variables|Default|GetHitBox) false false))

(event EventDestroyed
  (bind _asmain_game_mode (Utilities|Casting|CastToMainGameMode (Game|GetGameMode)))
  (Default|DoRespawn _asmain_game_mode self))

(event EventTick
  (params (DeltaSeconds :type Float%20%28single-precision%29))
  (if (not (Variables|Default|GetTaking%20Damage))
    (CallFunction|UpdateAnim)
    (if (Variables|Default|GetIs%20Sliding)
      (CallFunction|PushCheck)
      (Math|Float|CompareFloat (Math|Vector|VectorLength (Variables|/Script/Engine.MovementComponent|GetVelocity (Variables|Character|GetCharacterMovement))) 2e+01
        (:>
          (if (AI|Components|NavMovement|IsFalling (Variables|Character|GetCharacterMovement))
            (CallFunction|FinishSliding :!label _label)))
        (:==
          (goto _label))
        (:<
          (goto _label)))
      (elif (Variables|Default|GetIsAttacking)
        (if (and (== (Class|PaperFlipbookComponent|GetPlaybackPositioninFrames (Variables|Default|GetSprite)) 0) (Variables|Default|GetAtk%201))
          (Utilities|FlowControl|DoOnce false
            (:Completed
              (CallFunction|HitCheck1)))
          (elif (and (== (Class|PaperFlipbookComponent|GetPlaybackPositioninFrames (Variables|Default|GetSprite)) 10) (Variables|Default|GetAtk%202))
            (Utilities|FlowControl|DoOnce false
              (:Completed
                (CallFunction|HitCheck2)))))))))

(event Game|Damage|EventAnyDamage
  (params (Damage :type Float%20%28single-precision%29) (DamageType :type Damage%20Type%20Object%20Reference) (InstigatedBy :type Controller%20Object%20Reference) (DamageCauser :type Actor%20Object%20Reference))
  (bind _sprite (Variables|Default|GetSprite))
  (if (not (Variables|Default|GetTaking%20Damage))
    (Variables|Default|SetTaking%20Damage true)
    (if (not (Variables|Default|GetIs%20Dying))
      (Development|PrintText "Damage taken")
      (Variables|Default|SetHealth (- (Variables|Default|GetHealth) Damage))
      (if (<= (Variables|Default|GetHealth) 0.0)
        (Input|SetIgnoreMoveInput (Pawn|GetController) true)
        (Variables|/Script/Engine.MovementComponent|SetVelocity (Variables|Character|GetCharacterMovement) "0, 0, 0")
        (Variables|Default|SetIs%20Dying true)
        (Sprite|SetFlipbook _sprite "/Game/Assets/MainCharacter/Death/Death1.Death1")
        (Utilities|FlowControl|Delay (Class|PaperFlipbookComponent|GetFlipbookLength _sprite))
        (Development|PrintString "Dead")
        (Actor|DestroyActor)
        (else
          (Sprite|SetFlipbook (Variables|Default|GetSprite) "/Game/Assets/MainCharacter/Hurt/FB_MC_Hit.FB_MC_Hit")
          (Utilities|FlowControl|Delay (Class|PaperFlipbookComponent|GetFlipbookLength (Variables|Default|GetSprite)))
          (Variables|Default|SetTaking%20Damage false)
          (Sprite|SetFlipbook (Variables|Default|GetSprite) "/Game/Assets/MainCharacter/Idle/FB_Idle.FB_Idle"))))))

(event Custom|Finish%20Sliding
  (if (Variables|Default|GetIs%20Sliding)
    (Components|Capsule|SetCapsuleHalfHeight (Variables|Collision|GetCapsuleComponent) 2e+01 true)
    (Transformation|SetRelativeLocation (Variables|Default|GetSprite) "0.000000,0.000000,10.000000" false false)
    (Sprite|SetFlipbook (Variables|Default|GetSprite) "/Game/Assets/MainCharacter/Slide/FB_MC_SlideFin.FB_MC_SlideFin")
    (Utilities|FlowControl|Delay (Class|PaperFlipbookComponent|GetFlipbookLength (Variables|Default|GetSprite)))
    (Components|Timeline|SetLooping (Variables|Default|GetSprite) true)
    (Audio|Components|Audio|Play (Variables|Default|GetSprite))
    (Input|SetIgnoreMoveInput (Pawn|GetController) false)
    (Variables|Default|SetIs%20Sliding false)))

(event EventOnMovementModeChanged
  (params (PrevMovementMode :type EMovementMode%20Enum :default "MOVE_None") (NewMovementMode :type EMovementMode%20Enum :default "MOVE_None") (PrevCustomMode :type Byte :default 0) (NewCustomMode :type Byte :default 0))
  (if (and (Utilities|Enum|Equal(Enum) PrevMovementMode "MOVE_Falling") (Utilities|Enum|Equal(Enum) NewMovementMode "MOVE_Walking"))
    (if (Variables|Default|GetJump%20Buffered)
      (Character|Jump)
      (Variables|Default|SetJump%20Buffered false))
    (elif (and (Utilities|Enum|Equal(Enum) PrevMovementMode "MOVE_Walking") (Utilities|Enum|Equal(Enum) NewMovementMode "MOVE_Falling"))
      (Variables|Default|SetLedge%20Tolerant true)
      (Utilities|FlowControl|RetriggerableDelay 0.15)
      (Variables|Default|SetLedge%20Tolerant false))))

(event EventOnLanded
  (params (Hit :type Hit%20Result%20Structure%20%28by%20ref%29))
  (if (Variables|Default|GetIsAttacking)
    (Input|SetIgnoreMoveInput (Pawn|GetController) false)
    (CallFunction|SpawnHitShockwave)
    (CallFunction|DownHitCheck)
    (Variables|Default|SetIsAttacking false))
  (Math|Float|CompareFloat (.Z (Math|Vector|BreakVector (Variables|/Script/Engine.MovementComponent|GetVelocity (Variables|Character|GetCharacterMovement)))) -7.2e+02
    (:==
      _)
    (:<
      _))
  (CallFunction|SpawnDust))

(event Input|ActionEvents|InputActionJump
  (params (Key :type Key%20Structure :default "None"))
  (:Pressed
    (if (Variables|Default|GetIsAttacking)
      (if (Variables|Default|GetLedge%20Tolerant) :!label _label
        (Pawn|Components|CharacterMovement|SetMovementMode (Variables|Character|GetCharacterMovement) "MOVE_Walking" 0)
        (Character|Jump)
        (Variables|Default|SetLedge%20Tolerant false)
        (else
          (Variables|Default|SetJump%20Buffered true)
          (Utilities|FlowControl|RetriggerableDelay 0.2)
          (Variables|Default|SetJump%20Buffered false)))
      (elif (Character|CanJump)
        (Character|Jump)
        (else
          (goto _label)))))
  (:Released
    (Character|StopJumping)
    (Variables|Default|SetLedge%20Tolerant false)))

(event Input|ActionEvents|InputActionSlide
  (params (Key :type Key%20Structure :default "None"))
  (:Pressed
    (bind _can_slide (CallFunction|CanSlide))
    (if _can_slide
      (CallFunction|DecreaseDashQnt)
      (Variables|Default|SetIs%20Sliding true)
      (Components|Capsule|SetCapsuleHalfHeight (Variables|Collision|GetCapsuleComponent) 1e+01 true)
      (Transformation|SetRelativeLocation (Variables|Default|GetSprite) "0.000000,0.000000,15.000000" false false)
      (Input|SetIgnoreMoveInput (Pawn|GetController) true)
      (Physics|AddImpulse (Variables|Character|GetCharacterMovement) (Math|Vector|MakeVector (Variables|Default|GetLaunchX%20velocity) 0.0 0.0) true)
      (Sprite|SetFlipbook (Variables|Default|GetSprite) "/Game/Assets/MainCharacter/Slide/FB_MC_SlideStart.FB_MC_SlideStart")
      (Utilities|FlowControl|Delay (Class|PaperFlipbookComponent|GetFlipbookLength (Variables|Default|GetSprite)))
      (if (Variables|Default|GetIs%20Sliding)
        (Sprite|SetFlipbook (Variables|Default|GetSprite) "/Game/Assets/MainCharacter/Slide/FB_MC_SlideProcess.FB_MC_SlideProcess")))))

(event Input|AxisEvents|InputAxisMoveRight
  (params (AxisValue :type Float%20%28single-precision%29))
  (CallFunction|UpdateRotation)
  (Pawn|Input|AddMovementInput "1.000000,0.000000,0.000000" AxisValue false))

(event Custom|UpdateAnim
  (if (not (Variables|Default|GetIsAttacking))
    (if (not (Variables|Default|GetIs%20Sliding))
      (Sprite|SetFlipbook (Variables|Default|GetSprite) (select (AI|Components|NavMovement|IsFalling (Variables|Character|GetCharacterMovement)) "/Game/Assets/MainCharacter/Jump/FB_Jumping.FB_Jumping" (select (> (Math|Vector|VectorLength (Variables|/Script/Engine.MovementComponent|GetVelocity (Variables|Character|GetCharacterMovement))) 0.0) "/Game/Assets/MainCharacter/Running/FB_Running.FB_Running" "/Game/Assets/MainCharacter/Idle/FB_Idle.FB_Idle"))))))

(event Custom|UpdateRotation
  (Utilities|IsValid (Pawn|GetController)
    (:Is%20Valid
      (Math|Float|CompareFloat (.X (Math|Vector|BreakVector (Variables|/Script/Engine.MovementComponent|GetVelocity (Variables|Character|GetCharacterMovement)))) 0.0
        (:>
          (Variables|Default|SetLaunchX%20velocity 512.0)
          (Pawn|SetControlRotation (Pawn|GetController) (Math|Rotator|MakeRotator 0.0 0.0 0.0)))
        (:<
          (Variables|Default|SetLaunchX%20velocity -512.0)
          (Pawn|SetControlRotation (Pawn|GetController) (Math|Rotator|MakeRotator 0.0 0.0 1.8e+02)))))))

(event Input|ActionEvents|InputActionAttack
  (params (Key :type Key%20Structure :default "None"))
  (bind _capsulecomponent (Variables|Collision|GetCapsuleComponent))
  (bind _sprite (Variables|Default|GetSprite))
  (bind _sprite_2 (Variables|Default|GetSprite))
  (bind _capsulecomponent_2 (Variables|Collision|GetCapsuleComponent))
  (bind _returnvalue (Class|CapsuleComponent|GetUnscaledCapsuleRadius _capsulecomponent_2))
  (bind _returnvalue_2 (Transformation|GetWorldLocation _capsulecomponent))
  (bind _returnvalue_3 (Class|CapsuleComponent|GetUnscaledCapsuleRadius _capsulecomponent))
  (bind _returnvalue_4 (Transformation|GetWorldLocation _capsulecomponent_2))
  (bind _returnvalue_5 (- (.x _returnvalue_2) _returnvalue_3))
  (bind _returnvalue_6 (+ _returnvalue (.x _returnvalue_4)))
  (:Pressed
    (Variables|Default|Setis%20Second%20attack true)
    (if (not (Variables|Default|GetIsAttacking))
      (if (AI|Components|NavMovement|IsFalling (Variables|Character|GetCharacterMovement))
        (bind _outhit (Collision|LineTraceByChannel (Math|Vector|MakeVector _returnvalue_5 (.y _returnvalue_2) (.z _returnvalue_2)) (Math|Vector|MakeVector _returnvalue_5 (.y _returnvalue_2) (- (.z _returnvalue_2) 1e+03)) "TraceTypeQuery1" false 0 "None"))
        (Math|Float|CompareFloat (.Distance (Collision|BreakHitResult _outhit)) 1.5e+02
          (:>
            _)
          (:==
            _))
        (bind _outhit_2 (Collision|LineTraceByChannel (Math|Vector|MakeVector _returnvalue_6 (.y _returnvalue_4) (.z _returnvalue_4)) (Math|Vector|MakeVector _returnvalue_6 (.y _returnvalue_4) (- (.z _returnvalue_4) 1e+03)) "TraceTypeQuery1" false 0 "None"))
        (Math|Float|CompareFloat (.Distance (Collision|BreakHitResult _outhit_2)) 1.5e+02
          (:>
            _)
          (:==
            _))
        (Input|SetIgnoreMoveInput (Pawn|GetController) true)
        (Variables|/Script/Engine.MovementComponent|SetVelocity (Variables|Character|GetCharacterMovement) "0.000000,0.000000,-1000.000000")
        (Variables|Default|SetIsAttacking true)
        (Sprite|SetFlipbook (Variables|Default|GetSprite) "/Game/Assets/MainCharacter/AttackFalling/FB_FallingAttack_2.FB_FallingAttack_2")
        (elif (not (Variables|Default|GetIs%20Sliding))
          (Variables|Default|SetAtk%201 true)
          (Variables|Default|SetIsAttacking true)
          (Input|SetIgnoreMoveInput (Pawn|GetController) true)
          (Sprite|SetFlipbook _sprite "/Game/Assets/MainCharacter/Attack/FB_Attack_1.FB_Attack_1")
          (Utilities|FlowControl|Delay (Class|PaperFlipbookComponent|GetFlipbookLength _sprite))
          (if (Variables|Default|Getis%20Second%20attack)
            (Variables|Default|SetAtk%201 false)
            (Variables|Default|SetAtk%202 true)
            (CallFunction|ResetHit2)
            (Sprite|SetFlipbook _sprite_2 "/Game/Assets/MainCharacter/Attack/FB_MC_Attack_2.FB_MC_Attack_2")
            (Utilities|FlowControl|Delay (Class|PaperFlipbookComponent|GetFlipbookLength _sprite_2)))
          (Variables|Default|SetIsAttacking false)
          (Variables|Default|SetAtk%201 false)
          (Variables|Default|SetAtk%202 false)
          (Input|SetIgnoreMoveInput (Pawn|GetController) false)
          (CallFunction|ResetHit1)
          (CallFunction|ResetHit2)
          (if (Variables|Default|GetJump%20Buffered)
            (Character|Jump)
            (Variables|Default|SetJump%20Buffered false))))))
  (:Released
    (Variables|Default|Setis%20Second%20attack false)))

(fn ConstructionScript)

(fn HitCheck1
  (for _array_element (Collision|GetOverlappingActors (Variables|Default|GetFlatAttack%201) "/Game/Blueprints/BP_Skeleton.BP_Skeleton_C" :!class /Script/Engine.PrimitiveComponent)
    (if (!= _array_element self)
      (bind _returnvalue (Game|Damage|ApplyDamage _array_element (Variables|Default|GetDamage) 0 self))
      (Development|PrintText (Utilities|Text|ToText(Float) _returnvalue "HalfToEven")))))

(fn SpawnDust
  (bind _sprite (Variables|Default|GetSprite))
  (bind _returnvalue (Transformation|GetWorldTransform _sprite))
  (Game|SpawnActorfromClass "/Game/Assets/Effects/Landing/BP_Land.BP_Land_C" (Math|Transform|MakeTransform (.location _returnvalue) (.rotation _returnvalue) (.scale _returnvalue)) "Undefined" "MultiplyWithRoot" 0 0))

(fn DownHitCheck
  (for _array_element (Collision|GetOverlappingActors (Variables|Default|GetFallAttack) "/Game/Blueprints/BP_Skeleton.BP_Skeleton_C" :!class /Script/Engine.PrimitiveComponent)
    (if (!= _array_element self)
      (bind _returnvalue (Game|Damage|ApplyDamage _array_element (Variables|Default|GetDamage) 0 self))
      (Development|PrintText (Utilities|Text|ToText(Float) _returnvalue "HalfToEven")))))

(fn SpawnHitShockwave
  (bind _sprite (Variables|Default|GetSprite))
  (bind _sprite_2 (Variables|Default|GetSprite))
  (bind _returnvalue (Transformation|GetWorldTransform _sprite))
  (bind _returnvalue_2 (Transformation|GetWorldTransform _sprite_2))
  (Math|Float|CompareFloat (.z (Variables|/Script/Engine.MovementComponent|GetVelocity (Variables|Character|GetCharacterMovement))) -8e+02
    (:>
      (Game|SpawnActorfromClass "/Game/Assets/MainCharacter/AttackFalling/BP_ShockWaveLittle.BP_ShockWaveLittle_C" (Math|Transform|MakeTransform (.location _returnvalue) (.rotation _returnvalue) (.scale _returnvalue)) "Undefined" "MultiplyWithRoot" 0 0))
    (:==
      (Game|SpawnActorfromClass "/Game/Assets/MainCharacter/AttackFalling/BP_Shockwave.BP_Shockwave_C" (Math|Transform|MakeTransform (.location _returnvalue_2) (.rotation _returnvalue_2) (.scale _returnvalue_2)) "Undefined" "MultiplyWithRoot" 0 0 :!label _label))
    (:<
      (goto _label))))

(fn IncreaseDashQnt
  (Math|Integer|CompareInt (Variables|Default|GetSlide%20Qnt) 3
    (:<
      (Variables|Default|SetSlide%20Qnt (+ (Variables|Default|GetSlide%20Qnt) 1)))))

(fn CanSlide
  (if (or (AI|Components|NavMovement|IsFalling (Variables|Character|GetCharacterMovement)) (Variables|Default|GetIs%20Sliding))
    _
    (else
      (Math|Integer|CompareInt (Variables|Default|GetSlide%20Qnt)
        (:>
          (return true))
        (:==
          _)
        (:<
          _))))
  (return false))

(fn DecreaseDashQnt
  (Variables|Default|SetSlide%20Qnt (- (Variables|Default|GetSlide%20Qnt) 1))
  (Math|Integer|CompareInt (Variables|Default|GetSlide%20Qnt)
    (:<
      (Variables|Default|SetSlide%20Qnt 0))))

(fn PushCheck
  (for _array_element (Collision|GetOverlappingActors (Variables|Default|GetPushCollision) "/Game/Blueprints/BP_Skeleton.BP_Skeleton_C" :!class /Script/Engine.PrimitiveComponent)
    (if (!= _array_element self)
      (bind _asbp_skeleton (Utilities|Casting|CastToBP_Skeleton _array_element))
      (Physics|AddImpulse (Variables|/Script/Engine.Character|GetCharacterMovement _asbp_skeleton) (Math|Vector|MakeVector 0.0 0.0 (Math|Float|SafeDivide (Math|Float|Absolute(Float) (.x (Variables|/Script/Engine.MovementComponent|GetVelocity (Variables|Character|GetCharacterMovement)))) 2.0)) true))))

(fn HitCheck2
  (for _array_element (Collision|GetOverlappingActors (Variables|Default|GetFlatAttack%202) "/Game/Blueprints/BP_Skeleton.BP_Skeleton_C" :!class /Script/Engine.PrimitiveComponent)
    (if (!= _array_element self)
      (bind _returnvalue (Game|Damage|ApplyDamage _array_element (Variables|Default|GetDamage) 0 self))
      (Development|PrintText (Utilities|Text|ToText(Float) _returnvalue "HalfToEven")))))